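; BP_Things_CONTENT is a clickable actor that opens a content screen.
; Clicking its Clicker component pauses the game, then creates a CONTENT widget and adds it to the viewport.
; The default BeginPlay, overlap and Tick events are disabled, and the construction script only calls its parent.
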(event OnClicked(clicker)
  (params (TouchedComponent :type Primitive%20Component%20Object%20Reference) (ButtonPressed :type Key%20Structure))
  (Game|SetGamePaused true)
  (bind _returnvalue (UserInterface|CreateWidget "/Game/ThingsBP/CONTENT.CONTENT_C"))
  (UserInterface|Viewport|AddtoViewport _returnvalue 0))

(event EventBeginPlay
  (|CallParentFunction) ; This node is disabled and will not be called.\nDrag off pins to build functionality.
)

(event Collision|EventActorBeginOverlap
  (params (OtherActor :type Actor%20Object%20Reference))
  (|CallParentFunction OtherActor) ; This node is disabled and will not be called.\nDrag off pins to build functionality.
)

(event EventTick
  (params (DeltaSeconds :type Float%20%28single-precision%29))
  (|CallParentFunction DeltaSeconds) ; This node is disabled and will not be called.\nDrag off pins to build functionality.
)

(fn ConstructionScript
  (|CallParentFunction))