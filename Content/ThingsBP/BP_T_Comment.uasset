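; Interactable object Blueprint that shows a line of dialogue text on screen when InteractDialogue fires.
; On BeginPlay it caches the Objects_Data_act1 DataTable rows matching its ObjectID.
; DialogueGetLine filters those rows by ConversationID and LineCurrent, returning the text when ReturnedLines holds exactly one entry.
; Interaction toggles the dialogue widget, and a retriggerable delay removes it automatically.
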(event EventBeginPlay
  (|CallParentFunction)
  (bind _outrownames (DataTable|GetDataTableRowNames "/Game/Dialogues/Objects_Data_act1.Objects_Data_act1"))
  (for _array_element _outrownames
    (bind _returnvalue (Utilities|GetDataTableRow "/Game/Dialogues/Objects_Data_act1.Objects_Data_act1" _array_element)
      (:then
        (if (== (.Object_ID (Utilities|Struct|BreakDialogueStruct _returnvalue)) (Variables|Default|GetObject_ID))
          (Utilities|Array|Add (Variables|Default|GetDialogue) _array_element))))))

(event Collision|EventActorBeginOverlap
  (params (OtherActor :type Actor%20Object%20Reference))
  (|CallParentFunction OtherActor) ; This node is disabled and will not be called.\nDrag off pins to build functionality.
)

(event EventTick
  (params (DeltaSeconds :type Float%20%28single-precision%29))
  (|CallParentFunction DeltaSeconds) ; This node is disabled and will not be called.\nDrag off pins to build functionality.
)

(event EventInteractDialogue
  (Utilities|IsValid (Variables|Default|GetDialogueWidget)
    (:Is%20Valid
      (Widget|RemovefromParent (Variables|Default|GetDialogueWidget))
      (Variables|Default|SetDialogueWidget 0))
    (:Is%20Not%20Valid
      (bind _returnvalue (UserInterface|CreateWidget "/Game/Dialogues/DialogueWid.DialogueWid_C" (Game|GetPlayerController 0)))
      (bind _output_get (Variables|Default|SetDialogueWidget _returnvalue))
      (UserInterface|Viewport|AddtoViewport _output_get 0)
      (bind _returnedline (CallFunction|DialogueGetLine))
      (Variables|/Game/Dialogues/DialogueWid.DialogueWid_C|SetDialogueText (Variables|Default|GetDialogueWidget) _returnedline)
      (Utilities|FlowControl|RetriggerableDelay 1e+01)
      (Widget|RemovefromParent (Variables|Default|GetDialogueWidget))
      (Variables|Default|SetDialogueWidget 0))))

(fn ConstructionScript
  (|CallParentFunction))

(fn DialogueGetLine
  (for _array_element (Variables|Default|GetDialogue)
    (bind _returnvalue (Utilities|GetDataTableRow "/Game/Dialogues/Objects_Data_act1.Objects_Data_act1" _array_element)
      (:then
        (if (and (== (.Conversation_ID (Utilities|Struct|BreakDialogueStruct _returnvalue)) (Variables|Default|GetConversation_ID)) (== (.Line_ID (Utilities|Struct|BreakDialogueStruct _returnvalue)) (Variables|Default|GetLine_Current)))
          (Utilities|Array|Add (LocalVariables|GetReturnedLines) (.Dialogue (Utilities|Struct|BreakDialogueStruct _returnvalue)))))))
  (if (== (Utilities|Array|Length (LocalVariables|GetReturnedLines)) 1)
    (return (Utilities|Array|Get(acopy) (LocalVariables|GetReturnedLines)))))