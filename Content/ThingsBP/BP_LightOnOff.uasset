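; BP_LightOnOff is a clickable light switch that toggles a light and calms the Sanya character's fear.
; A trigger volume sets a Nearby flag while Sanya overlaps it, and clicking the sphere only works when that flag is set.
; A click calls the light's toggle, zeroes Sanya's fear state and calls its Fear function.
; BeginPlay caches the first Sanya and first BP_Light found in the level.
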(event OnClicked(Sphere)
  (params (TouchedComponent :type Primitive%20Component%20Object%20Reference) (ButtonPressed :type Key%20Structure))
  (bind _boyref (Variables|Default|GetBoyRef))
  (if (Variables|Default|GetNearby)
    (Default|TurnonOffLight (Variables|Default|GetLight))
    (Variables|/Game/BoyCharacter/Blueprints/Sanya.Sanya_C|SetFearInt _boyref 0)
    (Variables|/Game/BoyCharacter/Blueprints/Sanya.Sanya_C|SetFearOn? _boyref false)
    (Default|Fear _boyref)))

(event OnComponentBeginOverlap(Trigg)
  (params (OverlappedComponent :type Primitive%20Component%20Object%20Reference) (OtherActor :type Actor%20Object%20Reference) (OtherComp :type Primitive%20Component%20Object%20Reference) (OtherBodyIndex :type Integer) (bFromSweep :type Boolean) (SweepResult :type Hit%20Result%20Structure%20%28by%20ref%29))
  (Utilities|Casting|CastToSanya OtherActor)
  (Variables|Default|SetNearby true))

(event OnComponentEndOverlap(Trigg)
  (params (OverlappedComponent :type Primitive%20Component%20Object%20Reference) (OtherActor :type Actor%20Object%20Reference) (OtherComp :type Primitive%20Component%20Object%20Reference) (OtherBodyIndex :type Integer))
  (Utilities|Casting|CastToSanya OtherActor)
  (Variables|Default|SetNearby false))

(event Collision|EventActorBeginOverlap
  (params (OtherActor :type Actor%20Object%20Reference)))

(event EventTick
  (params (DeltaSeconds :type Float%20%28single-precision%29)))

(event EventBeginPlay
  (bind _outactors (Actor|GetAllActorsOfClass "/Game/BoyCharacter/Blueprints/Sanya.Sanya_C"))
  (Variables|Default|SetBoyRef (Utilities|Array|Get(acopy) _outactors))
  (bind _outactors_2 (Actor|GetAllActorsOfClass "/Game/ThingsBP/BP_Light.BP_Light_C"))
  (Variables|Default|SetLight (Utilities|Array|Get(acopy) _outactors_2)))

(fn ConstructionScript)