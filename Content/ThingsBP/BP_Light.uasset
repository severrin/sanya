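; BP_Light is a toggleable light actor that starts switched off and tells the Sanya character when it is dark.
; BeginPlay caches the first BP_LightOnOff and Sanya, then calls TurnOnOffLight.
; That event flips three point lights, shows the switch actor's two cubes while dark, and updates Sanya's LightOff flag.
; Trigger overlap events are empty, leaving the fear, panic and dog-order logic disconnected.
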(event OnComponentBeginOverlap(FearTrigger)
  (params (OverlappedComponent :type Primitive%20Component%20Object%20Reference) (OtherActor :type Actor%20Object%20Reference) (OtherComp :type Primitive%20Component%20Object%20Reference) (OtherBodyIndex :type Integer) (bFromSweep :type Boolean) (SweepResult :type Hit%20Result%20Structure%20%28by%20ref%29)))

(event OnComponentEndOverlap(FearTrigger)
  (params (OverlappedComponent :type Primitive%20Component%20Object%20Reference) (OtherActor :type Actor%20Object%20Reference) (OtherComp :type Primitive%20Component%20Object%20Reference) (OtherBodyIndex :type Integer)))

(event OnComponentBeginOverlap(StopTrigger)
  (params (OverlappedComponent :type Primitive%20Component%20Object%20Reference) (OtherActor :type Actor%20Object%20Reference) (OtherComp :type Primitive%20Component%20Object%20Reference) (OtherBodyIndex :type Integer) (bFromSweep :type Boolean) (SweepResult :type Hit%20Result%20Structure%20%28by%20ref%29)))

(event OnComponentBeginOverlap(Stop2)
  (params (OverlappedComponent :type Primitive%20Component%20Object%20Reference) (OtherActor :type Actor%20Object%20Reference) (OtherComp :type Primitive%20Component%20Object%20Reference) (OtherBodyIndex :type Integer) (bFromSweep :type Boolean) (SweepResult :type Hit%20Result%20Structure%20%28by%20ref%29)))

(event OnComponentBeginOverlap(Dog)
  (params (OverlappedComponent :type Primitive%20Component%20Object%20Reference) (OtherActor :type Actor%20Object%20Reference) (OtherComp :type Primitive%20Component%20Object%20Reference) (OtherBodyIndex :type Integer) (bFromSweep :type Boolean) (SweepResult :type Hit%20Result%20Structure%20%28by%20ref%29)))

(event Custom|TurnOnOffLight
  (bind _light (Variables|Default|Getlight))
  (bind _boyref (Variables|Default|GetBoyRef))
  (bind _pointlight (Variables|Default|GetPointLight))
  (bind _cube (Variables|/Game/ThingsBP/BP_LightOnOff.BP_LightOnOff_C|GetCube _light))
  (if (Variables|Default|GetLightOn?)
    (Rendering|SetVisibility _pointlight false false)
    (Rendering|SetVisibility _cube true false)
    (Variables|Default|SetLightOn? false)
    (Variables|/Game/BoyCharacter/Blueprints/Sanya.Sanya_C|SetLightOff? _boyref true)
    (else
      (Rendering|SetVisibility _pointlight true false)
      (Rendering|SetVisibility _cube false false)
      (Variables|Default|SetLightOn? true)
      (Variables|/Game/BoyCharacter/Blueprints/Sanya.Sanya_C|SetLightOff? _boyref false))))

(event EventBeginPlay
  (Variables|Default|SetLightOn? true)
  (bind _outactors (Actor|GetAllActorsOfClass "/Game/ThingsBP/BP_LightOnOff.BP_LightOnOff_C"))
  (Variables|Default|Setlight (Utilities|Array|Get(acopy) _outactors))
  (bind _outactors_2 (Actor|GetAllActorsOfClass "/Game/BoyCharacter/Blueprints/Sanya.Sanya_C"))
  (Variables|Default|SetBoyRef (Utilities|Array|Get(acopy) _outactors_2))
  (CallFunction|TurnonOffLight))

(event Collision|EventActorBeginOverlap
  (params (OtherActor :type Actor%20Object%20Reference)))

(event EventTick
  (params (DeltaSeconds :type Float%20%28single-precision%29)))

(fn ConstructionScript)