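; Clickable cassette pickup that flags the level's BP_T_CommentPLAYER as having the cassette and shows a text comment.
; Clicking messages every InteractInterface actor overlapping Sanya, whose reference is cached on collision overlap.
; Interacting plays a click, hides the sprite and shows a dialogue widget, then removes both widget and actor after a retriggerable delay; interacting again closes the widget.
; Data-table dialogue lookup logic is present but never runs.
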(event OnComponentBeginOverlap(Collision)
  (params (OverlappedComponent :type Primitive%20Component%20Object%20Reference) (OtherActor :type Actor%20Object%20Reference) (OtherComp :type Primitive%20Component%20Object%20Reference) (OtherBodyIndex :type Integer) (bFromSweep :type Boolean) (SweepResult :type Hit%20Result%20Structure%20%28by%20ref%29))
  (bind _assanya (Utilities|Casting|CastToSanya OtherActor))
  (Variables|Default|SetSanyaRef _assanya))

(event OnComponentEndOverlap(Collision)
  (params (OverlappedComponent :type Primitive%20Component%20Object%20Reference) (OtherActor :type Actor%20Object%20Reference) (OtherComp :type Primitive%20Component%20Object%20Reference) (OtherBodyIndex :type Integer))
  (Utilities|Casting|CastToSanya OtherActor))

(event OnClicked(clicker)
  (params (TouchedComponent :type Primitive%20Component%20Object%20Reference) (ButtonPressed :type Key%20Structure))
  (bind _outactors (Actor|GetAllActorswithInterface "/Game/Dialogues/InteractInterface.InteractInterface_C"))
  (for _array_element _outactors
    (if (Collision|IsOverlappingActor _array_element (Variables|Default|GetSanyaRef) :!class /Script/Engine.Actor)
      (Class|InteractInterface|InteractDialogue(Message) _array_element))))

(event EventBeginPlay
  (|CallParentFunction))

(event Collision|EventActorBeginOverlap
  (params (OtherActor :type Actor%20Object%20Reference))
  (|CallParentFunction OtherActor) ; This node is disabled and will not be called.\nDrag off pins to build functionality.
)

(event EventTick
  (params (DeltaSeconds :type Float%20%28single-precision%29))
  (|CallParentFunction DeltaSeconds) ; This node is disabled and will not be called.\nDrag off pins to build functionality.
)

(event EventInteractDialogue
  (Audio|PlaySound2D "/Game/Sounds/Click.Click" 1.0 1.0 0.0 0 0)
  (bind _outactors (Actor|GetAllActorsOfClass "/Game/ThingsBP/BP_T_CommentPLAYER.BP_T_CommentPLAYER_C"))
  (Variables|/Game/ThingsBP/BP_T_CommentPLAYER.BP_T_CommentPLAYER_C|SetCassette (Utilities|Array|Get(acopy) _outactors) true)
  (Utilities|IsValid (Variables|Default|GetDialogueWidget)
    (:Is%20Valid
      (Widget|RemovefromParent (Variables|Default|GetDialogueWidget))
      (Variables|Default|SetDialogueWidget 0))
    (:Is%20Not%20Valid
      (bind _returnvalue (UserInterface|CreateWidget "/Game/Dialogues/DialogueWid.DialogueWid_C" (Game|GetPlayerController 0)))
      (bind _output_get (Variables|Default|SetDialogueWidget _returnvalue))
      (UserInterface|Viewport|AddtoViewport _output_get 0)
      (Variables|/Game/Dialogues/DialogueWid.DialogueWid_C|SetDialogueText (Variables|Default|GetDialogueWidget) (Variables|Default|GetText))
      (Rendering|SetVisibility (Variables|Default|GetPaperSprite) false false)
      (Utilities|FlowControl|RetriggerableDelay 1e+01)
      (Widget|RemovefromParent (Variables|Default|GetDialogueWidget))
      (Variables|Default|SetDialogueWidget 0)
      (Actor|DestroyActor))))

(fn ConstructionScript
  (|CallParentFunction))

(fn DialogueGetLine
  (for _array_element (Variables|Default|GetDialogue)
    (bind _returnvalue (Utilities|GetDataTableRow "/Game/Dialogues/Objects_Data_act1.Objects_Data_act1" _array_element)
      (:then
        (if (and (== (.Conversation_ID (Utilities|Struct|BreakDialogueStruct _returnvalue)) (Variables|Default|GetConversation_ID)) (== (.Line_ID (Utilities|Struct|BreakDialogueStruct _returnvalue)) (Variables|Default|GetLine_Current)))
          (Utilities|Array|Add (LocalVariables|GetReturnedLines) (.Dialogue (Utilities|Struct|BreakDialogueStruct _returnvalue)))))))
  (if (== (Utilities|Array|Length (LocalVariables|GetReturnedLines)) 1)
    (return (Utilities|Array|Get(acopy) (LocalVariables|GetReturnedLines)))))