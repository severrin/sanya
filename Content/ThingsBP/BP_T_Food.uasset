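; Food pickup actor that the Sanya character can take by clicking on it while nearby.
; The Collision component sets a CanTake flag when Sanya begins overlapping and clears it when Sanya leaves.
; A click on the Clicker component, if allowed, assigns this actor as Sanya's Food and calls TakeFood on SanyaRef.
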(event OnClicked(Sphere)
  (params (TouchedComponent :type Primitive%20Component%20Object%20Reference) (ButtonPressed :type Key%20Structure)))

(event OnClicked(clicker)
  (params (TouchedComponent :type Primitive%20Component%20Object%20Reference) (ButtonPressed :type Key%20Structure))
  (bind _sanyaref (Variables|Default|GetSanyaRef))
  (if (Variables|Default|GetCanTake?)
    (Variables|/Game/BoyCharacter/Blueprints/Sanya.Sanya_C|SetFood _sanyaref self)
    (Default|TakeFood _sanyaref)))

(event OnComponentBeginOverlap(Collision)
  (params (OverlappedComponent :type Primitive%20Component%20Object%20Reference) (OtherActor :type Actor%20Object%20Reference) (OtherComp :type Primitive%20Component%20Object%20Reference) (OtherBodyIndex :type Integer) (bFromSweep :type Boolean) (SweepResult :type Hit%20Result%20Structure%20%28by%20ref%29))
  (Utilities|Casting|CastToSanya OtherActor)
  (CallFunction|CanTake))

(event OnComponentEndOverlap(Collision)
  (params (OverlappedComponent :type Primitive%20Component%20Object%20Reference) (OtherActor :type Actor%20Object%20Reference) (OtherComp :type Primitive%20Component%20Object%20Reference) (OtherBodyIndex :type Integer))
  (Utilities|Casting|CastToSanya OtherActor)
  (Variables|Default|SetCanTake? false))

(event Custom|CanTake
  (Variables|Default|SetCanTake? true))

(event EventBeginPlay)

(event Collision|EventActorBeginOverlap
  (params (OtherActor :type Actor%20Object%20Reference)))

(event EventTick
  (params (DeltaSeconds :type Float%20%28single-precision%29)))

(fn ConstructionScript)