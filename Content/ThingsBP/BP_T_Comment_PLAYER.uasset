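; Interactable cassette player that gives a comment when used and, if HaveCassette is set, toggles between flat ambient sound and a Sonic music track.
; Ambient 2D audio starts on BeginPlay, and each toggle stops the current sound and spawns the other, tracked by the Sound flag.
; After music starts, a retriggerable delay later spawns the ambient sound again and clears the flag.
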(event Custom|SoundOnOff
  (if (Variables|Default|GetSound?)
    (Audio|Components|Audio|Stop (Variables|Default|GetSonicSound))
    (bind _returnvalue (Audio|SpawnSound2D "/Game/Sounds/Ambient/AmbientFlat.AmbientFlat" 1.0 1.0 0.0 0))
    (Variables|Default|SetFlatSound _returnvalue)
    (Variables|Default|SetSound? false)
    (else
      (Audio|Components|Audio|Stop (Variables|Default|GetFlatSound))
      (bind _returnvalue_2 (Audio|SpawnSound2D "/Game/Sounds/SonicCue.SonicCue" 1.0 1.0 0.0 0))
      (Variables|Default|SetSonicSound _returnvalue_2)
      (Variables|Default|SetSound? true)
      (Utilities|FlowControl|RetriggerableDelay 4.2e+02)
      (bind _returnvalue_3 (Audio|SpawnSound2D "/Game/Sounds/Ambient/AmbientFlat.AmbientFlat" 1.0 1.0 0.0 0))
      (Variables|Default|SetFlatSound _returnvalue_3)
      (Variables|Default|SetSound? false))))

(event EventBeginPlay
  (|CallParentFunction)
  (bind _returnvalue (Audio|SpawnSound2D "/Game/Sounds/Ambient/AmbientFlat.AmbientFlat" 1.0 1.0 0.0 0 false false))
  (Variables|Default|SetFlatSound _returnvalue))

(event Collision|EventActorBeginOverlap
  (params (OtherActor :type Actor%20Object%20Reference))
  (|CallParentFunction OtherActor) ; This node is disabled and will not be called.\nDrag off pins to build functionality.
)

(event EventTick
  (params (DeltaSeconds :type Float%20%28single-precision%29))
  (|CallParentFunction DeltaSeconds) ; This node is disabled and will not be called.\nDrag off pins to build functionality.
)

(event EventInteractDialogue
  (CallFunction|Comment)
  (if (Variables|Default|GetHaveCassette)
    (CallFunction|SoundonOff)))

(fn ConstructionScript
  (|CallParentFunction))