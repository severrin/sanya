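; Hallway dialogue trigger that, on Sanya's first overlap, disables input and creates a DialogueWidHALL choice widget.
; Unless Run is set, it shows the widget and fills in the main text, two answers and Fin.
; A separate Runing event auto-walks Sanya along +X, re-arming a short timer and switching animation until a threshold X is passed.
; The ambient hallway sound node is left unconnected.
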(event OnComponentBeginOverlap(Trigger)
  (params (OverlappedComponent :type Primitive%20Component%20Object%20Reference) (OtherActor :type Actor%20Object%20Reference) (OtherComp :type Primitive%20Component%20Object%20Reference) (OtherBodyIndex :type Integer) (bFromSweep :type Boolean) (SweepResult :type Hit%20Result%20Structure%20%28by%20ref%29))
  (bind _returnvalue (Game|GetPlayerController 0))
  (bind _assanya (Utilities|Casting|CastToSanya OtherActor))
  (Utilities|FlowControl|Sequence
    (:then_0
      (Utilities|FlowControl|DoOnce false
        (:Completed
          (Input|DisableInput _assanya _returnvalue)
          (bind _returnvalue_2 (UserInterface|CreateWidget "/Game/Dialogues/Hallway/DialogueWidHALL.DialogueWidHALL_C" _returnvalue))
          (bind _output_get (Variables|Default|SetWidgetDialogue _returnvalue_2))
          (if (Variables|Default|GetRun)
            (Widget|RemovefromParent _output_get)
            (else
              (UserInterface|Viewport|AddtoViewport _output_get 0)
              (Variables|/Game/Dialogues/Hallway/DialogueWidHALL.DialogueWidHALL_C|SetDialogueText (Variables|Default|GetWidgetDialogue) (Variables|Default|GetMainText))
              (Variables|/Game/Dialogues/Hallway/DialogueWidHALL.DialogueWidHALL_C|SetAnswerTextOne (Variables|Default|GetWidgetDialogue) (Variables|Default|GetAnswerOne))
              (Variables|/Game/Dialogues/Hallway/DialogueWidHALL.DialogueWidHALL_C|SetAnswerTextTwo (Variables|Default|GetWidgetDialogue) (Variables|Default|GetAnswerTwo))
              (Variables|/Game/Dialogues/Hallway/DialogueWidHALL.DialogueWidHALL_C|SetFin (Variables|Default|GetWidgetDialogue) (Variables|Default|GetFin)))))))))

(event Custom|Runing
  (bind _outactors (Actor|GetAllActorsOfClass "/Game/BoyCharacter/Blueprints/Sanya.Sanya_C"))
  (Pawn|Input|AddMovementInput (Utilities|Array|Get(acopy) _outactors) "1.000000, 0, 0" 3.0 true)
  (Variables|/Script/Engine.CharacterMovementComponent|SetMaxWalkSpeed (Variables|/Script/Engine.Character|GetCharacterMovement (Utilities|Array|Get(acopy) _outactors)) 4e+02)
  (if (> (.x (Transformation|GetActorLocation (Utilities|Array|Get(acopy) _outactors))) 646.0)
    (Variables|/Game/BoyCharacter/Blueprints/Sanya.Sanya_C|SetAnimations (Utilities|Array|Get(acopy) _outactors) "NewEnumerator4")
    (else
      (Utilities|Time|SetTimerbyEvent (delegate Custom|Runing) 0.001)
      (Variables|/Game/BoyCharacter/Blueprints/Sanya.Sanya_C|SetAnimations (Utilities|Array|Get(acopy) _outactors) "NewEnumerator2"))))

(event EventBeginPlay)

(event Collision|EventActorBeginOverlap
  (params (OtherActor :type Actor%20Object%20Reference)))

(event EventTick
  (params (DeltaSeconds :type Float%20%28single-precision%29)))

(fn ConstructionScript)